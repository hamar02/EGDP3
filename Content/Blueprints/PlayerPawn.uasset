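; Player-controlled 2D pawn with a Paper2D flipbook that moves on the world XY plane.
; MoveRight and MoveUp axis inputs fill a Movement vector, which Tick scales by MoveSpeed and delta time.
; Each axis is applied as a separate swept offset, and horizontal direction flips the flipbook by setting its world rotation.
; The Attack input calls an Attack function that is still empty.
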(event `InputAxis|MoveRight`
  (params (AxisValue :type "Float (single-precision)"))
  (set `self.Movement` (`KismetMathLibrary.MakeVector2D` AxisValue (`.Y` (`KismetMathLibrary.BreakVector2D` (`self.Movement`))))))

(event `InputAxis|MoveUp`
  (params (AxisValue :type "Float (single-precision)"))
  (set `self.Movement` (`KismetMathLibrary.MakeVector2D` (`KismetMathLibrary.BreakVector2D` (`self.Movement`)) AxisValue)))

(event `self.ReceiveTick`
  (params (DeltaSeconds :type "Float (single-precision)"))
  (bind _movespeed (`self.MoveSpeed`))
  (bind _paperflipbook (`self.PaperFlipbook`))
  (bind _x (`KismetMathLibrary.BreakVector2D` (`self.Movement`)))
  (bind (_x_2 _y) (`KismetMathLibrary.BreakVector2D` (`self.Movement`)))
  (`self.K2_AddActorWorldOffset` (* (* (`KismetMathLibrary.MakeVector` _x_2) _movespeed) DeltaSeconds) true)
  (`self.K2_AddActorWorldOffset` (* (* (`KismetMathLibrary.MakeVector` 0.0 _y) _movespeed) DeltaSeconds) true)
  (if (> _x 0.0)
    (`SceneComponent.K2_SetWorldRotation` :`self` _paperflipbook)
    (elif (< _x 0.0)
      (`SceneComponent.K2_SetWorldRotation` _paperflipbook (struct :`Yaw` 180.0) false false))))

(event `InputAction|Attack`
  (params (Key :type "Key Structure"))
  (:`Pressed`
    (`self.Attack`)))

(fn `Attack`)

(fn `UserConstructionScript`)