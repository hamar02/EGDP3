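; TerrainSection is a Paper2D terrain piece with a building and road that randomizes its look and populates itself with NPCs.
; The construction script picks a random building sprite, then randomizes child decal sprites, drawing building children from RoadDecals and road children from BuildingDecals.
; Decal index ranges include the array length, so a pick can fall out of bounds.
; On BeginPlay it spawns a small random number of NPCPawns at random horizontal offsets around itself.
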(event `self.ReceiveBeginPlay`
  (for _ (range (+ (`KismetMathLibrary.RandomIntegerInRange` 1 3) 1))
    (`|SpawnActorFromClass` "/Game/Blueprints/NPCPawn.NPCPawn_C" (`KismetMathLibrary.MakeTransform` (+ (.location (`self.GetTransform` self)) (`KismetMathLibrary.MakeVector` (`KismetMathLibrary.RandomFloatInRange` -1000.0 1000.0) (`KismetMathLibrary.RandomFloatInRange` -1000.0 1000.0))) (.rotation (`self.GetTransform` self)) (.scale (`self.GetTransform` self))) "Undefined" "OverrideRootScale" null null)))

(fn `UserConstructionScript`
  (bind _buildingsprites (`self.BuildingSprites`))
  (bind _roaddecals (`self.RoadDecals`))
  (bind _buildingdecals (`self.BuildingDecals`))
  ;[1 1 1] Random building
  (`PaperSpriteComponent.SetSprite` (`self.PaperSpriteBuilding`) (`|GetArrayItem` _buildingsprites (`KismetMathLibrary.RandomIntegerInRange` 0 (- (`KismetArrayLibrary.Array_Length` _buildingsprites) 1))))
  ;[1 1 1] Random building decals
  (for _array_element (`SceneComponent.GetChildrenComponents` (`self.PaperSpriteBuilding`) false)
    (bind _aspaper_sprite_component (cast `PaperSpriteComponent` _array_element))
    (`PaperSpriteComponent.SetSprite` _aspaper_sprite_component (`|GetArrayItem` _roaddecals (`KismetMathLibrary.RandomIntegerInRange` 0 (`KismetArrayLibrary.Array_Length` _roaddecals)))))
  ;[1 1 1] Random road decals
  (for _array_element_2 (`SceneComponent.GetChildrenComponents` (`self.PaperSpriteRoad`) false)
    (bind _aspaper_sprite_component_2 (cast `PaperSpriteComponent` _array_element_2))
    (`PaperSpriteComponent.SetSprite` _aspaper_sprite_component_2 (`|GetArrayItem` _buildingdecals (`KismetMathLibrary.RandomIntegerInRange` 0 (`KismetArrayLibrary.Array_Length` _buildingdecals))))))