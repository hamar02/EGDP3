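; NPCPawn is a Paper2D NPC pawn with movement, facing, a melee attack and health.
; Tick applies the clamped Movement vector as separate swept X and Y offsets scaled by MoveSpeed, and rotates the flipbook to face horizontal travel.
; Attack sphere-traces on the facing side using AttackRange, but its hits are unused.
; Damage lowers Health within a zero-to-one range and destroys the actor at zero.
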(event `self.ReceiveTick`
  (params (DeltaSeconds :type "Float (single-precision)"))
  (bind _movespeed (`self.MoveSpeed`))
  (bind _paperflipbook (`self.PaperFlipbook`))
  (bind _x (`KismetMathLibrary.BreakVector2D` (`self.Movement`)))
  (bind (_x_2 _y) (`KismetMathLibrary.BreakVector2D` (`self.Movement`)))
  (`self.K2_AddActorWorldOffset` (* (* (`KismetMathLibrary.MakeVector` (`KismetMathLibrary.FClamp` _x_2 -1.0)) _movespeed) DeltaSeconds) true)
  (`self.K2_AddActorWorldOffset` (* (* (`KismetMathLibrary.MakeVector` 0.0 (`KismetMathLibrary.FClamp` _y -1.0)) _movespeed) DeltaSeconds) true)
  (if (> _x 0.0)
    (`SceneComponent.K2_SetWorldRotation` :`self` _paperflipbook)
    (set `self.FacingRight` true)
    (elif (< _x 0.0)
      (`SceneComponent.K2_SetWorldRotation` _paperflipbook (struct :`Yaw` 180.0) false false)
      (set `self.FacingRight` false))))

(fn `Attack`
  (bind _returnvalue (* (`self.AttackRange`) 0.5))
  (bind _returnvalue_2 (+ (`self.K2_GetActorLocation`) (`KismetMathLibrary.MakeVector` (select `bool` (`self.FacingRight`) :`false` (* _returnvalue -1.0) :`true` _returnvalue))))
  (`KismetSystemLibrary.SphereTraceMultiForObjects` _returnvalue_2 _returnvalue_2 _returnvalue (`|MakeArray` "ObjectTypeQuery7" "ObjectTypeQuery8" :!type "EObjectTypeQuery Enum")))

(fn `Damage`
  (params (Amount :type "Float (double-precision)"))
  (bind _output_get (set `self.Health` (`KismetMathLibrary.FClamp` (- (`self.Health`) Amount))))
  (if (<= _output_get 0.0)
    (`self.K2_DestroyActor`)))

(fn `UserConstructionScript`)