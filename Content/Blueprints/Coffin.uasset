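; Coffin is a 2D sprite actor that bursts apart ten seconds after BeginPlay or upon taking any damage, then triggers the game's end screen.
; Both triggers share one sequence that spawns separate upper and lower coffin pieces at offset positions, plays a particle burst and removes the sprite.
; After a short delay it deactivates the emitter, calls EndScreen on the side-scroller game mode and destroys itself.
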(event `self.ReceiveBeginPlay`
  (bind _returnvalue (`self.GetTransform`))
  (bind _returnvalue_2 (`self.GetTransform`))
  (bind _returnvalue_3 (`KismetMathLibrary.TransformRotation` _returnvalue))
  (bind _returnvalue_4 (`KismetMathLibrary.TransformLocation` _returnvalue))
  (`KismetSystemLibrary.Delay` 10.0)
  (`|SpawnActorFromClass` "/Game/Blueprints/CoffinUpper.CoffinUpper_C" (`KismetMathLibrary.MakeTransform` (+ (`KismetMathLibrary.TransformLocation` _returnvalue_2) (-100.0 0.0 100.0)) (`KismetMathLibrary.TransformRotation` _returnvalue_2)) "AlwaysSpawn" "OverrideRootScale" null null :!label _label)
  (`|SpawnActorFromClass` "/Game/Blueprints/CoffinLower.CoffinLower_C" (`KismetMathLibrary.MakeTransform` (+ _returnvalue_4 (100.0 0.0 -100.0)) _returnvalue_3) "AlwaysSpawn" "OverrideRootScale" null null)
  (bind _returnvalue_5 (`GameplayStatics.SpawnEmitterAtLocation` "/Game/Particles/WhaamCoffinParticleSystem.WhaamCoffinParticleSystem" _returnvalue_4 _returnvalue_3))
  (`ActorComponent.K2_DestroyComponent` (`self.PaperSprite`))
  (`KismetSystemLibrary.Delay` 0.5)
  (`ActorComponent.Deactivate` _returnvalue_5)
  (bind _as2dside_scroller_game_mode (cast `/Game/Blueprints/2DSideScrollerGameMode` (`GameplayStatics.GetGameMode`)))
  (`/Game/Blueprints/2DSideScrollerGameMode.End Screen` _as2dside_scroller_game_mode)
  (`self.K2_DestroyActor`))

(event `self.ReceiveAnyDamage`
  (params (Damage :type "Float (single-precision)") (DamageType :type "DamageType Object Reference") (InstigatedBy :type "Controller Object Reference") (DamageCauser :type "Actor Object Reference"))
  (goto _label))

(fn `UserConstructionScript`)